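; BP_Enemy is an enemy actor that flies in a straight line and destroys the player on contact.
; At BeginPlay it picks a fixed direction, with a 30% chance toward the player's position at that moment, otherwise its own forward vector.
; Tick moves it through a frame-rate-independent Translate function and turns it to face that direction.
; Overlapping BP_Player spawns an explosion, destroys both actors and plays a sound.
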(event `self.ReceiveBeginPlay`
  ;[1 1 1] 적이 태어날 때(BeginPlay) 진행 방향을 30% 확률은 플레이어를 향하게 한다. 나머지 70% 확률은 전진 방향(타겟-나)으로 정하고 싶다.
  (if (< (`KismetMathLibrary.RandomIntegerInRange` 0 9) 3)
    ;;[1 1 1] 적이 플레이어를 찾아서 그 방향을 구한 후  Direction 변수에  넣어 그 방향으로 다가간다.
    (set `self.Direction` (`KismetMathLibrary.Normal` (- (`self.K2_GetActorLocation` (`GameplayStatics.GetPlayerPawn` 0)) (`self.K2_GetActorLocation`))))
    (else
      (set `self.Direction` (`self.GetActorForwardVector`)))))

(event `self.ReceiveTick`
  (params (DeltaSeconds :type "Float (single-precision)"))
  (`self.Translate` (`self.Direction`) (`self.Speed`))
  (`self.K2_SetActorRotation` (`KismetMathLibrary.MakeRotFromXZ` (`self.Direction`) (`self.GetActorUpVector`))))

(event `self.ReceiveActorBeginOverlap`
  (params (OtherActor :type "Actor Object Reference"))
  (bind _asbp_player (cast `/Game/BP_Player` OtherActor))
  (`GameplayStatics.SpawnEmitterAtLocation` "/Game/StarterContent/Particles/P_Explosion.P_Explosion" (`self.K2_GetActorLocation` _asbp_player))
  (`self.K2_DestroyActor` _asbp_player)
  (`self.K2_DestroyActor`)
  (`GameplayStatics.PlaySound2D` "/Game/Resource/destruction.destruction" 1.0 1.0 0.0 null null))

(fn `Translate`
  (params (Direction :type "Vector Structure") (Speed :type "Float (double-precision)") (NewParam :type Boolean))
  (`self.K2_SetActorLocation` (+ (`self.K2_GetActorLocation`) (* (`KismetMathLibrary.Normal` Direction) Speed (`GameplayStatics.GetWorldDeltaSeconds`)))))

(fn `UserConstructionScript`)