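; Enemy spawner actor that periodically creates BP_Enemy instances in the level.
; On BeginPlay it starts a looping timer at the MakeTime interval that calls MakeEnemy, which spawns the enemy at the Arrow component's transform regardless of collision.
; An older Tick-based accumulator doing the same job is left disconnected and never runs.
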(event `self.ReceiveBeginPlay`
  (`KismetSystemLibrary.K2_SetTimer` null "MakeEnemy" (`self.MakeTime`) true))

(event `self.ReceiveTick`
  (params (DeltaSeconds :type "Float (single-precision)"))
  ;[1 1 1] 시간이 흐르다가 현재 시간이 생성 시간이 되면 적을 Arrow 위치에 Spawn 하고 싶다. 그리고 현재 시간을 0 으로 초기화 하고 싶다.
)

(fn `MakeEnemy`
  (`|SpawnActorFromClass` "/Game/BP_Enemy.BP_Enemy_C" (`SceneComponent.K2_GetComponentToWorld` (`self.Arrow`)) "AlwaysSpawn" "MultiplyWithRoot" null null))

(fn `UserConstructionScript`)