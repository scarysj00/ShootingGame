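; BP_Bullet is a projectile actor that destroys enemies on contact and awards score.
; Each tick, a Translate function moves it along its forward vector by Speed and delta time, teleport and sweep off.
; On overlapping a BP_Enemy, it spawns an explosion at the enemy, destroys both actors and plays a destruction sound.
; It then adds one point through BP_ShootingGameModeBase.
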(event `self.ReceiveActorBeginOverlap`
  (params (OtherActor :type "Actor Object Reference"))
  (bind _asbp_enemy (cast `/Game/BP_Enemy` OtherActor))
  (`GameplayStatics.SpawnEmitterAtLocation` "/Game/StarterContent/Particles/P_Explosion.P_Explosion" (`self.K2_GetActorLocation` _asbp_enemy))
  (`self.K2_DestroyActor` _asbp_enemy)
  (`self.K2_DestroyActor`)
  (`GameplayStatics.PlaySound2D` "/Game/Resource/destruction.destruction" 1.0 1.0 0.0 null null)
  (bind _asbp_shooting_game_mode_base (cast `/Game/BP_ShootingGameModeBase` (`GameplayStatics.GetGameMode`)))
  (`/Game/BP_ShootingGameModeBase.AddScore` _asbp_shooting_game_mode_base 1))

(event `self.ReceiveTick`
  (params (DeltaSeconds :type "Float (single-precision)"))
  (`self.Translate` (`self.GetActorForwardVector`) (`self.Speed`)))

(fn `Translate`
  (params (Direction :type "Vector Structure") (Speed :type "Float (double-precision)") (NewParam :type Boolean))
  (`self.K2_SetActorLocation` (+ (`self.K2_GetActorLocation`) (* (`KismetMathLibrary.Normal` Direction) Speed (`GameplayStatics.GetWorldDeltaSeconds`)))))

(fn `UserConstructionScript`)