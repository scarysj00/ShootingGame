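; BP_Player is the player actor that moves on the Y-Z plane and fires bullets.
; Enhanced Input axes feed Horizontal and Vertical, which Tick normalizes and scales by Speed and delta time to set location without sweep.
; Holding fire spawns BP_Bullet at the Arrow transform immediately, then on a looping timer until release clears it.
; An older Delay-based auto-fire branch with a laser sound is never run.
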(event `self.ReceiveBeginPlay`
  (`EnhancedInputSubsystemInterface.AddMappingContext` (pcsubsystem `EnhancedInputLocalPlayerSubsystem` (`GameplayStatics.GetPlayerController` 0)) "/Game/Input/IMC_Player.IMC_Player" 0 (struct)))

(event `EnhancedInput|/Game/Input/IA_Horizontal`
  (params (ActionValue :type "Float (double-precision)") (ElapsedSeconds :type "Float (double-precision)") (TriggeredSeconds :type "Float (double-precision)") (InputAction :type "InputAction Object Reference" :default "/Game/Input/IA_Horizontal.IA_Horizontal"))
  (:`Triggered`
    (set `self.Horizontal` ActionValue))
  (:`Completed`
    (set `self.Horizontal` ActionValue)))

(event `EnhancedInput|/Game/Input/IA_Vertical`
  (params (ActionValue :type "Float (double-precision)") (ElapsedSeconds :type "Float (double-precision)") (TriggeredSeconds :type "Float (double-precision)") (InputAction :type "InputAction Object Reference" :default "/Game/Input/IA_Vertical.IA_Vertical"))
  (:`Triggered`
    (set `self.Vertical` ActionValue))
  (:`Completed`
    (set `self.Vertical` ActionValue)))

(event `self.ReceiveTick`
  (params (DeltaSeconds :type "Float (single-precision)"))
  (`|ExecutionSequence`
    (:`then_0`
      ;[1 1 1] 사용자의 입력에 따라 이동하고 싶다. P = P0 + VT
      (`self.K2_SetActorLocation` (+ (`self.K2_GetActorLocation`) (* (* (`KismetMathLibrary.Normal` (`KismetMathLibrary.MakeVector` 0.0 (`self.Horizontal`) (`self.Vertical`))) (`self.Speed`)) DeltaSeconds))))))

(event `EnhancedInput|/Game/Input/IA_Fire`
  (params (ActionValue :type Boolean) (ElapsedSeconds :type "Float (double-precision)") (TriggeredSeconds :type "Float (double-precision)") (InputAction :type "InputAction Object Reference" :default "/Game/Input/IA_Fire.IA_Fire"))
  (:`Started`
    (bind _returnvalue (`KismetSystemLibrary.K2_SetTimer` null "MakeBullet" (`self.FireInterval`) true))
    (set `self.MakeBulletTimerHandle` _returnvalue)
    (`self.MakeBullet`))
  (:`Completed`
    (`KismetSystemLibrary.K2_ClearAndInvalidateTimerHandle` (`self.MakeBulletTimerHandle`))))

(fn `MakeBullet`
  (`|SpawnActorFromClass` "/Game/BP_Bullet.BP_Bullet_C" (`SceneComponent.K2_GetComponentToWorld` (`self.Arrow`)) "AlwaysSpawn" "MultiplyWithRoot" null null))

(fn `UserConstructionScript`)